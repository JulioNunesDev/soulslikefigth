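; Inventory component that creates the master UI widget and manages its health, mana and effect potion slots.
; On BeginPlay it adds WB_Master_UI to the viewport, caches the three slot widgets and fills each with texture, type and count from PotionTable rows and stored Max variables.
; Update events increment a slot's potion count and copy it back to the matching Max variable, so the widgets hold the working count.
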(event EventBeginPlay
  (Utilities|FlowControl|Sequence
    (:then_0
      (bind _returnvalue (UserInterface|CreateWidget "/Game/Game/Components/Inventory/WB_Master_UI.WB_Master_UI_C"))
      (bind _output_get (Variables|Default|SetWB_Inventory_UI _returnvalue))
      (Variables|Default|SetHealth%20Slot (Variables|/Game/Game/Components/Inventory/WB_Master_UI.WB_Master_UI_C|GetHealthSlot _output_get))
      (Variables|Default|SetEffect%20Slot%201 (Variables|/Game/Game/Components/Inventory/WB_Master_UI.WB_Master_UI_C|GeteffectSlot_1 _output_get))
      (Variables|Default|SetMana%20Slot (Variables|/Game/Game/Components/Inventory/WB_Master_UI.WB_Master_UI_C|GetManaSlot _output_get))
      (UserInterface|Viewport|AddtoViewport _output_get 0))
    (:then_1
      (bind _returnvalue_2 (Utilities|GetDataTableRow "/Game/Game/BluePrints/World/Table/PotionTable.PotionTable" "Health")
        (:then
          ;[1 1 1] Set Health
          (Utilities|IsValid (Variables|Default|GetHealth%20Slot)
            (:Is%20Valid
              (Variables|/Game/Game/Components/Inventory/WB_Inventory_SLot.WB_Inventory_SLot_C|SetTextureImage (Variables|Default|GetHealth%20Slot) (.ImageTexture (Utilities|Struct|BreakPotionStruct _returnvalue_2)))
              (Variables|/Game/Game/Components/Inventory/WB_Inventory_SLot.WB_Inventory_SLot_C|SetPotionNumber (Variables|Default|GetHealth%20Slot) (Variables|Default|GetMaxPotionHealth))
              (Variables|/Game/Game/Components/Inventory/WB_Inventory_SLot.WB_Inventory_SLot_C|SetType (Variables|Default|GetHealth%20Slot) (.TypePotion (Utilities|Struct|BreakPotionStruct _returnvalue_2))))))))
    (:then_2
      (bind _returnvalue_3 (Utilities|GetDataTableRow "/Game/Game/BluePrints/World/Table/PotionTable.PotionTable" "Mana")
        (:then
          ;[1 1 1] Set Mana
          (Utilities|IsValid (Variables|Default|GetMana%20Slot)
            (:Is%20Valid
              (Variables|/Game/Game/Components/Inventory/WB_Inventory_SLot.WB_Inventory_SLot_C|SetTextureImage (Variables|Default|GetMana%20Slot) (.ImageTexture (Utilities|Struct|BreakPotionStruct _returnvalue_3)))
              (Variables|/Game/Game/Components/Inventory/WB_Inventory_SLot.WB_Inventory_SLot_C|SetPotionNumber (Variables|Default|GetMana%20Slot) (Variables|Default|GetMaxPotionMana))
              (Variables|/Game/Game/Components/Inventory/WB_Inventory_SLot.WB_Inventory_SLot_C|SetType (Variables|Default|GetMana%20Slot) (.TypePotion (Utilities|Struct|BreakPotionStruct _returnvalue_3))))))))
    (:then_3
      (bind _returnvalue_4 (Utilities|GetDataTableRow "/Game/Game/BluePrints/World/Table/PotionTable.PotionTable" "Effect")
        (:then
          ;[1 1 1] Set Health
          (Utilities|IsValid (Variables|Default|GetEffect%20Slot%201)
            (:Is%20Valid
              (Variables|/Game/Game/Components/Inventory/WB_Inventory_SLot.WB_Inventory_SLot_C|SetTextureImage (Variables|Default|GetEffect%20Slot%201) (.ImageTexture (Utilities|Struct|BreakPotionStruct _returnvalue_4)))
              (Variables|/Game/Game/Components/Inventory/WB_Inventory_SLot.WB_Inventory_SLot_C|SetPotionNumber (Variables|Default|GetEffect%20Slot%201) (Variables|Default|GetMaxPotionEffect))
              (Variables|/Game/Game/Components/Inventory/WB_Inventory_SLot.WB_Inventory_SLot_C|SetType (Variables|Default|GetEffect%20Slot%201) (.TypePotion (Utilities|Struct|BreakPotionStruct _returnvalue_4))))))))))

(event EventUpdateHealth
  (bind _health_slot (Variables|Default|GetHealth%20Slot))
  ;[1 1 1] Logic Add Health
  (Utilities|IsValid _health_slot
    (:Is%20Valid
      (bind _output_get (Variables|/Game/Game/Components/Inventory/WB_Inventory_SLot.WB_Inventory_SLot_C|SetPotionNumber _health_slot (+ (Variables|/Game/Game/Components/Inventory/WB_Inventory_SLot.WB_Inventory_SLot_C|GetPotionNumber _health_slot) 1.0)))
      (Variables|Default|SetMaxPotionHealth _output_get))))

(event EventUpdateMana
  (bind _mana_slot (Variables|Default|GetMana%20Slot))
  ;[1 1 1] Logic Add Health
  (Utilities|IsValid _mana_slot
    (:Is%20Valid
      (bind _output_get (Variables|/Game/Game/Components/Inventory/WB_Inventory_SLot.WB_Inventory_SLot_C|SetPotionNumber _mana_slot (+ (Variables|/Game/Game/Components/Inventory/WB_Inventory_SLot.WB_Inventory_SLot_C|GetPotionNumber _mana_slot) 1.0)))
      (Variables|Default|SetMaxPotionMana _output_get))))

(event EventUpdateEffect
  (bind _effect_slot_1 (Variables|Default|GetEffect%20Slot%201))
  ;[1 1 1] Logic Add Health
  (Utilities|IsValid _effect_slot_1
    (:Is%20Valid
      (bind _output_get (Variables|/Game/Game/Components/Inventory/WB_Inventory_SLot.WB_Inventory_SLot_C|SetPotionNumber _effect_slot_1 (+ (Variables|/Game/Game/Components/Inventory/WB_Inventory_SLot.WB_Inventory_SLot_C|GetPotionNumber _effect_slot_1) 1.0)))
      (Variables|Default|SetMaxPotionEffect _output_get))))